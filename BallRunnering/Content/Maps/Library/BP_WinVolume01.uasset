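; BP_WinVolume01 is a level-exit trigger that lets the player finish once all crystals are collected.
; On player overlap, it prints a Polish warning if any Gem or Gem2 actors remain.
; Otherwise it fades the camera, waits, then opens the level following the current one in TabLevelNames.
; A final-level flag is queried but does not alter the flow, and the next index is not bounds-checked.
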(event OnComponentBeginOverlap(Box)
  (params (OverlappedComponent :type Primitive%20Component%20Object%20Reference) (OtherActor :type Actor%20Object%20Reference) (OtherComp :type Primitive%20Component%20Object%20Reference) (OtherBodyIndex :type Integer) (bFromSweep :type Boolean) (SweepResult :type Hit%20Result%20Structure%20%28by%20ref%29))
  (Utilities|IsPlayer OtherActor
    (:true
      (bind _outactors (Actor|GetAllActorsOfClass "/Game/Maps/Library/Gem.Gem_C"))
      (bind _outactors_2 (Actor|GetAllActorsOfClass "/Game/Maps/Library/Gem2.Gem2_C"))
      (if (or (> (Utilities|Array|Length _outactors_2) 0) (> (Utilities|Array|Length _outactors) 0))
        (Development|PrintString "Nie zebrano wszystkich kryształów")
        (else
          (CallFunction|CompleteLevel)
          (CameraFades|StartCameraFade (Game|GetPlayerCameraManager 0) 0.0 1.0 1.0 "(R=0.037429,G=0.000000,B=0.437500,A=1.000000)" false true)
          (Utilities|FlowControl|Delay 1.0)
          (CallFunction|LoadNextLevel))))))

(fn ConstructionScript)

(fn CompleteLevel
  (bind _checklastlevel (CallFunction|IsFinalLevel))
  (if (not _checklastlevel)
    (return)))

(fn IsFinalLevel
  (return (Variables|Default|GetCheckLastLevel)))

(fn GetCurrentLevelIndex
  (bind _returnvalue (Game|GetCurrentLevelName true))
  (return (Utilities|Array|FindItem (Variables|Default|Gettab_LevelNames) _returnvalue)))

(fn LoadNextLevel
  (bind _nextlevelname (CallFunction|GetNextLevelName))
  (CallFunction|IsFinalLevel)
  (Game|OpenLevel(byName) (Utilities|String|StringToName _nextlevelname)))

(fn GetNextLevelName
  (bind _levelindex (CallFunction|GetCurrentLevelIndex))
  (return (Utilities|Array|Get(acopy) (Variables|Default|Gettab_LevelNames) (+ _levelindex 1))))