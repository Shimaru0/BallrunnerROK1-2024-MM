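; BP_Ball01 is a player-controlled rolling ball that restarts the level when it takes damage.
; Both movement input axes drive a shared torque node on the Sphere, scaled by StrMultiply and applied as an acceleration change.
; Camera fades frame each attempt: from black on BeginPlay, and to red with a hurt sound on any damage, before the current level reloads after a short delay.
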(event Game|Damage|EventAnyDamage
  (params (Damage :type Float%20%28single-precision%29) (DamageType :type Damage%20Type%20Object%20Reference) (InstigatedBy :type Controller%20Object%20Reference) (DamageCauser :type Actor%20Object%20Reference))
  (Audio|PlaySound2D "/Game/Maps/mystuff/Audio/classic_hurt.classic_hurt" 1.0 1.0 0.0 0 0)
  (CameraFades|StartCameraFade (Game|GetPlayerCameraManager 0) 0.0 1.0 0.3 "(R=1.000000,G=0.000000,B=0.000000,A=1.000000)" false true)
  (Utilities|FlowControl|Delay 1.0)
  (bind _returnvalue (Game|GetCurrentLevelName true))
  (Game|OpenLevel(byName) (Utilities|String|StringToName _returnvalue)))

(event EventBeginPlay
  (CameraFades|StartCameraFade (Game|GetPlayerCameraManager 0) 1.0 0.0 0.3 "(R=0.000000,G=0.000000,B=0.000000,A=1.000000)" false true))

(event Input|AxisEvents|InputAxisMoveForwardBack
  (params (AxisValue :type Float%20%28single-precision%29))
  (bind _strmultiply (Variables|BallProperties|GetStrMultiply))
  (Class|PrimitiveComponent|AddTorqueinRadians (Variables|Default|GetSphere) (Math|Vector|MakeVector (* (stale Input|AxisEvents|InputAxisMoveLeftRight AxisValue) _strmultiply) (* AxisValue _strmultiply) 0.0) "None" true))

(event Input|AxisEvents|InputAxisMoveLeftRight
  (params (AxisValue :type Float%20%28single-precision%29))
  (bind _strmultiply (Variables|BallProperties|GetStrMultiply))
  (Class|PrimitiveComponent|AddTorqueinRadians (Variables|Default|GetSphere) (Math|Vector|MakeVector (* AxisValue _strmultiply) (* (stale Input|AxisEvents|InputAxisMoveForwardBack AxisValue) _strmultiply) 0.0) "None" true))

(fn ConstructionScript)