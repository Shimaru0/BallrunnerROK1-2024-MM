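; BP_Crystal_04 is a collectible crystal pickup that flies into the player when something overlaps its sphere.
; The overlap plays the Crystaltransform timeline, which lerps the crystal from its current location toward player pawn 0 while shrinking its scale to zero.
; When the timeline finishes, the actor destroys itself and plays the 2D Orb sound.
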(event OnComponentBeginOverlap(Sphere)
  (params (OverlappedComponent :type Primitive%20Component%20Object%20Reference) (OtherActor :type Actor%20Object%20Reference) (OtherComp :type Primitive%20Component%20Object%20Reference) (OtherBodyIndex :type Integer) (bFromSweep :type Boolean) (SweepResult :type Hit%20Result%20Structure%20%28by%20ref%29))
  (bind (_direction _location _size) (Timeline|crystaltransform Play)
    (:Update
      (Transformation|SetActorLocation (Math|Vector|Lerp(Vector) (Transformation|GetActorLocation) (Transformation|GetActorLocation (Game|Player|GetPlayerPawn 0)) _location) false false)
      (Transformation|SetActorScale3D (Math|Vector|Lerp(Vector) (Transformation|GetActorScale3D) "0, 0, 0" _size)))
    (:Finished
      (Actor|DestroyActor)
      (Audio|PlaySound2D "/Game/Maps/mystuff/Audio/orb.orb" 1.0 1.0 0.0 0 0))))

(fn ConstructionScript)